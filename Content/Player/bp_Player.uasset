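; Player Blueprint that handles first-person movement input.
; On BeginPlay it adds the FirstPersonControls Enhanced Input mapping context to its player controller's local subsystem.
; Forward, back and strafe input actions each pass the capsule component's forward or right vector, negated for back and left, to MoveDirection, whose body is not defined in these graphs.
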(event Input|EnhancedActionEvents|EnhancedInputActionmoveForward
  (params (ActionValue :type Boolean) (ElapsedSeconds :type Float%20%28double-precision%29) (TriggeredSeconds :type Float%20%28double-precision%29) (InputAction :type Input%20Action%20Object%20Reference :default "/Game/Controls/moveForward.moveForward"))
  ;[0.15 0.15 0.15 0.5] PlayerMovement
  (Class|PlayerCharacter|MoveDirection (Math|Vector|GetForwardVector (Variables|Default|GetCapsuleComponent))))

(event Input|EnhancedActionEvents|EnhancedInputActionmoveBack
  (params (ActionValue :type Boolean) (ElapsedSeconds :type Float%20%28double-precision%29) (TriggeredSeconds :type Float%20%28double-precision%29) (InputAction :type Input%20Action%20Object%20Reference :default "/Game/Controls/moveBack.moveBack"))
  ;[0.15 0.15 0.15 0.5] PlayerMovement
  (Class|PlayerCharacter|MoveDirection (Math|Vector|NegateVector (Math|Vector|GetForwardVector (Variables|Default|GetCapsuleComponent)))))

(event Input|EnhancedActionEvents|EnhancedInputActionstrafeLeft
  (params (ActionValue :type Boolean) (ElapsedSeconds :type Float%20%28double-precision%29) (TriggeredSeconds :type Float%20%28double-precision%29) (InputAction :type Input%20Action%20Object%20Reference :default "/Game/Controls/strafeLeft.strafeLeft"))
  ;[0.15 0.15 0.15 0.5] PlayerMovement
  (Class|PlayerCharacter|MoveDirection (Math|Vector|NegateVector (Math|Vector|GetRightVector (Variables|Default|GetCapsuleComponent)))))

(event Input|EnhancedActionEvents|EnhancedInputActionstrafeRight
  (params (ActionValue :type Boolean) (ElapsedSeconds :type Float%20%28double-precision%29) (TriggeredSeconds :type Float%20%28double-precision%29) (InputAction :type Input%20Action%20Object%20Reference :default "/Game/Controls/strafeRight.strafeRight"))
  ;[0.15 0.15 0.15 0.5] PlayerMovement
  (Class|PlayerCharacter|MoveDirection (Math|Vector|GetRightVector (Variables|Default|GetCapsuleComponent))))

(event EventBeginPlay
  (bind _asplayer_controller (Utilities|Casting|CastToPlayerController (Pawn|GetController)))
  (Utilities|IsValid (PlayerController|LocalPlayerSubsystems|GetEnhancedInputLocalPlayerSubsystem _asplayer_controller)
    (:Is%20Valid
      (Input|AddMappingContext (PlayerController|LocalPlayerSubsystems|GetEnhancedInputLocalPlayerSubsystem _asplayer_controller) "/Game/Controls/FirstPersonControls.FirstPersonControls" 0 "(bIgnoreAllPressedKeysUntilRelease=True,bForceImmediately=False,bNotifyUserSettings=False)"))))

(fn ConstructionScript)